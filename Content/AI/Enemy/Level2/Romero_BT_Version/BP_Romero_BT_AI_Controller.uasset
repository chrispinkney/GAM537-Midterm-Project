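; AI controller for the Romero enemy in its Behavior Tree version.
; On BeginPlay it caches the controlled pawn, runs Romero_BT, stores the player character as its target and writes the current state to the AIState blackboard key.
; A looping Test timer repeatedly forces that state to one fixed value, with no decision logic.
; A Pawn_Attack event forwards attack requests to the pawn.
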(event Custom|Pawn_Attack
  (Default|Attack (Variables|Default|GetRomero_Pawn)))

(event Custom|Test
  (bind _output_get (Variables|Default|SetCurrentState "NewEnumerator1"))
  (AI|Components|Blackboard|SetValueasEnum (AI|GetBlackboard 0) (Utilities|Name|MakeLiteralName "AIState") _output_get))

(event EventBeginPlay
  (bind _asbp_romero_bt1 (Utilities|Casting|CastToBP_Romero_BT1 (Pawn|GetControlledPawn)))
  (Variables|Default|SetRomero_Pawn _asbp_romero_bt1)
  (AI|RunBehaviorTree "/Game/AI/Enemy/Level2/Romero_BT_Version/Romero_BT.Romero_BT")
  (Variables|Default|SetCurrentTarget (Game|GetPlayerCharacter 0))
  (AI|Components|Blackboard|SetValueasEnum (AI|GetBlackboard 0) (Utilities|Name|MakeLiteralName "AIState") (Variables|Default|GetCurrentState))
  (Utilities|Time|SetTimerbyEvent (delegate Custom|Test) 0.5 true))

(fn ConstructionScript)